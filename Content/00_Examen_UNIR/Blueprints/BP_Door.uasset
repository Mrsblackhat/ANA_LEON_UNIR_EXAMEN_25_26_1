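; BP_Door is a sliding double door that other logic opens and closes through its OpenDoor and CloseDoor events.
; BeginPlay caches the starting relative locations of the right and left door components.
; A Timeline plays forward to lerp the two panels apart along local X in opposite directions, and plays in reverse to close them.
; The Blueprint has no trigger logic of its own, as its overlap and Tick events are disabled.
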(event `self.ReceiveBeginPlay`
  (set `self.IniPosR` (`SceneComponent.RelativeLocation` (`self.RDoor`)))
  (set `self.IniPosL` (`SceneComponent.RelativeLocation` (`self.LDoor`))))

(event `OpenDoor`
  (bind (_direction _newtrack_0) (`Timeline|Timeline` :!label _label)
    (:`Update`
      (`SceneComponent.K2_SetRelativeLocation` (`self.RDoor`) (`KismetMathLibrary.VLerp` (`self.IniPosR`) (+ (`self.IniPosR`) (80.0 0.0 0.0)) _newtrack_0) false false)
      (`SceneComponent.K2_SetRelativeLocation` (`self.LDoor`) (`KismetMathLibrary.VLerp` (`self.IniPosL`) (+ (`self.IniPosL`) (-80.0 0.0 0.0)) _newtrack_0) false false))))

(event `CloseDoor`
  (goto _label :!via `Reverse`))

(fn `UserConstructionScript`)