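; BP_FloorButton is a floor button that opens and closes a linked Door and swaps the material on its hieroglyph mesh.
; Pressing E latches a pressed flag, fires OnPressedChanged and toggles both door and material, without checking overlap or Door validity.
; Collision overlap resets the door and light state flags, then runs the same toggle if Door is valid and E was ever pressed.
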(event `self.Collision.OnComponentBeginOverlap`
  (params (OverlappedComponent :type "PrimitiveComponent Object Reference") (OtherActor :type "Actor Object Reference") (OtherComp :type "PrimitiveComponent Object Reference") (OtherBodyIndex :type Integer) (bFromSweep :type Boolean) (SweepResult :type "HitResult Structure (by ref)"))
  (bind _door (`self.Door`))
  (set `self.puertaAbierta` false)
  (set `self.encendido` false)
  (`/Engine/EditorBlueprintResources/StandardMacros.IsValid` _door
    (:`Is Valid`
      (if (stale `Key|E` _output_get) :!label _label
        (if (`self.puertaAbierta`)
          (`/Game/00_Examen_UNIR/Blueprints/BP_Door.CloseDoor` _door)
          (set `self.puertaAbierta` false)
          (else
            (`/Game/00_Examen_UNIR/Blueprints/BP_Door.OpenDoor` _door)
            (set `self.puertaAbierta` true)))
        (if (`self.encendido`)
          (set `self.encendido` false)
          (`PrimitiveComponent.SetMaterial` (`self.SM_hieroglyph_007`) 0 "/Game/LowPolyAssets/Materials/M_Emission_Platform.M_Emission_Platform")
          (else
            (set `self.encendido` true)
            (`PrimitiveComponent.SetMaterial` (`self.SM_hieroglyph_007`) 0 "/Engine/BasicShapes/BasicShapeMaterial.BasicShapeMaterial")))))))

(event `Key|E`
  (params (Key :type "Key Structure"))
  (:`Pressed`
    (bind _output_get (set `self.presionado` true))
    (`self.OnPressedChanged`)
    (goto _label)))

(fn `UserConstructionScript`)